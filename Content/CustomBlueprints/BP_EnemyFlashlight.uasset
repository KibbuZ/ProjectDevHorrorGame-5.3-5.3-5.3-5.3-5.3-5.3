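; Enemy flashlight Blueprint that lights up the player, setting their LightLevel and CanBeSeen flag.
; Overlapping LightRange starts a short Delay loop that line-traces visibility to the player and applies inverse-square falloff to SpotLight intensity.
; Blocked traces leave the last values intact; the loop clears them once the player leaves range.
; Neither write happens while the player's own flashlight is on.
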(event OnComponentBeginOverlap(LightRange)
  (params (OverlappedComponent :type Primitive%20Component%20Object%20Reference) (OtherActor :type Actor%20Object%20Reference) (OtherComp :type Primitive%20Component%20Object%20Reference) (OtherBodyIndex :type Integer) (bFromSweep :type Boolean) (SweepResult :type Hit%20Result%20Structure%20%28by%20ref%29))
  (bind _returnvalue (Game|GetPlayerCharacter 0))
  ;[1 1 1] Get Brightness Of Player Character In Light
  (if (== OtherActor _returnvalue)
    (if (Collision|IsOverlappingActor (Variables|Default|GetLight%20Range) _returnvalue :!class /Script/Engine.PrimitiveComponent) :!label _label
      (bind _outhit (Collision|LineTraceByChannel (Transformation|GetActorLocation) (Transformation|GetActorLocation (Game|GetPlayerCharacter 0)) "TraceTypeQuery1" false 0 "None" true "(R=1.000000,G=0.000000,B=0.000000,A=1.000000)" "(R=0.000000,G=1.000000,B=0.000000,A=1.000000)" 0.0))
      (if (== (.HitActor (Collision|BreakHitResult _outhit)) (Game|GetPlayerCharacter 0))
        (bind _asbp_top_down_character (Utilities|Casting|CastToBP_TopDownCharacter (Game|GetPlayerCharacter 0)))
        (if (Variables|/Game/TopDown/Blueprints/BP_TopDownCharacter.BP_TopDownCharacter_C|GetFlashlight%20On _asbp_top_down_character)
          _
          (else
            (Variables|/Game/TopDown/Blueprints/BP_TopDownCharacter.BP_TopDownCharacter_C|SetLight%20Level _asbp_top_down_character (* (Variables|/Script/Engine.LightComponentBase|GetIntensity (Variables|Default|GetSpotLight)) (/ 1.0 (* (.Distance (Collision|BreakHitResult _outhit)) (.Distance (Collision|BreakHitResult _outhit))))))
            (Variables|/Game/TopDown/Blueprints/BP_TopDownCharacter.BP_TopDownCharacter_C|SetCan%20Be%20Seen _asbp_top_down_character true))))
      (Utilities|FlowControl|Delay 0.2)
      (goto _label)
      (else
        (bind _asbp_top_down_character_2 (Utilities|Casting|CastToBP_TopDownCharacter (Game|GetPlayerCharacter 0)))
        (if (not (Variables|/Game/TopDown/Blueprints/BP_TopDownCharacter.BP_TopDownCharacter_C|GetFlashlight%20On _asbp_top_down_character_2))
          (Variables|/Game/TopDown/Blueprints/BP_TopDownCharacter.BP_TopDownCharacter_C|SetLight%20Level _asbp_top_down_character_2 0.0)
          (Variables|/Game/TopDown/Blueprints/BP_TopDownCharacter.BP_TopDownCharacter_C|SetCan%20Be%20Seen _asbp_top_down_character_2 false)
          (Development|PrintString "Player Left Flashlight"))))))

(fn ConstructionScript)