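; Mini enemy AI for Level 3 Room 3-1 that roams a fixed route and chases the player on sight.
; From BeginPlay, Patrol chains AI MoveTo calls through three destinations, out and back, looping on success.
; PawnSensing triggers ChasePawn and a negative sound cue, raising walk speed and moving toward the player.
; A failed chase resumes patrol without resetting speed; the FollowPawn graph is empty.
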(event OnSeePawn(PawnSensing)
  (params (Pawn :type Pawn%20Object%20Reference))
  ;[1 1 1] Chase Player
  (CallFunction|ChasePawn)
  (Audio|PlaySound2D "/Engine/VREditor/Sounds/VR_negative_Cue.VR_negative_Cue" 1.0 1.0 0.0 0 0))

(event Custom|Patrol
  ;[1 1 1] Roam
  (AI|AIMoveTo self (Variables|Default|GetDestination) 0 5.0 false
    (:OnSuccess
      (AI|AIMoveTo self (Variables|Default|GetDestination_0) 0 5.0 false
        (:OnSuccess
          (AI|AIMoveTo self (Variables|Default|GetDestination_1) 0 5.0 false
            (:OnSuccess
              (AI|AIMoveTo self (Variables|Default|GetDestination_0) 0 5.0 false
                (:OnSuccess
                  (CallFunction|Patrol))))))))))

(event Custom|Chase%20Pawn
  ;[1 1 1] Chase Player
  (Variables|/Script/Engine.CharacterMovementComponent|SetMaxWalkSpeed (Variables|Character|GetCharacterMovement) 9e+02)
  (AI|AIMoveTo self "0, 0, 0" (Game|GetPlayerCharacter 0) 0.0 false
    (:OnFail
      (CallFunction|Patrol))))

(event EventBeginPlay
  (CallFunction|Patrol))

(fn ConstructionScript)

(fn FollowPawn)