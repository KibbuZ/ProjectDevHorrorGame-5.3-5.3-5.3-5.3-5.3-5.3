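; BP_AI_Lv3_R3_Librarian is an enemy AI, the level 3 Librarian, that wanders until it sees a pawn and then chases the player.
; From BeginPlay it loops AI MoveTo calls to random reachable points within a radius of itself.
; PawnSensing sight plays a negative VR cue and starts a move toward player 0, whichever pawn was seen.
; A failed chase falls back to roaming, while a successful one triggers nothing further.
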(event OnSeePawn(PawnSensing)
  (params (Pawn :type Pawn%20Object%20Reference))
  ;[1 1 1] Chase Player
  (CallFunction|FollowPawn)
  (Audio|PlaySound2D "/Engine/VREditor/Sounds/VR_negative_Cue.VR_negative_Cue" 1.0 1.0 0.0 0 0))

(event Custom|follow%20pawn
  ;[1 1 1] Chase Player
  (AI|AIMoveTo self "0, 0, 0" (Game|GetPlayerCharacter 0) 0.0 false
    (:OnFail
      (CallFunction|Roam))))

(event Custom|Roam
  ;[1 1 1] Roam
  (AI|AIMoveTo self (.RandomLocation (AI|Navigation|GetRandomReachablePointinRadius (Transformation|GetActorLocation self) 2e+03 0 0)) 0 5.0 false
    (:OnSuccess
      _)
    (:OnFail
      _))
  (CallFunction|Roam))

(event EventBeginPlay
  (CallFunction|Roam))

(fn ConstructionScript)