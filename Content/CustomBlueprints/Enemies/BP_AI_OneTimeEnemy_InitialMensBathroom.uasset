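; Enemy AI for the initial men's bathroom encounter that guards its spawn point with an attached flashlight, investigating noises with a look-around sweep.
; PawnSensing sightings inside its vision cone build suspicion from the player's light level until a chase starts.
; A repeating line trace tracks the chased player, with a timer returning the enemy to its post.
; A player inside the takedown box can ragdoll it and disable its sight.
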(event OnHearNoise(PawnSensing)
  (params (Instigator :type Pawn%20Object%20Reference) (Location :type Vector%20%28by%20ref%29 :default "0, 0, 0") (Volume :type Float%20%28single-precision%29))
  (bind _capsulecomponent (Variables|Collision|GetCapsuleComponent))
  (bind _returnvalue (Transformation|GetWorldLocation _capsulecomponent))
  (bind _returnvalue_2 (Transformation|GetWorldRotation _capsulecomponent))
  ;[1 1 1] Hear Noise
  (AI|AIMoveTo self Location 0 2e+01 false :!label _label
    (:OnSuccess
      (Components|MoveComponentTo (Variables|Collision|GetCapsuleComponent) _returnvalue (Math|Rotator|MakeRotator (.roll _returnvalue_2) (.pitch _returnvalue_2) (+ (.yaw _returnvalue_2) 85.0)) false false 2.0 true)
      (Components|MoveComponentTo (Variables|Collision|GetCapsuleComponent) _returnvalue (Math|Rotator|MakeRotator (.roll _returnvalue_2) (.pitch _returnvalue_2) (- (.yaw _returnvalue_2) 1.7e+02)) false false 2.0 true)
      (Utilities|FlowControl|Sequence
        (:then_0
          (Utilities|FlowControl|DoOnce false ; enters at Reset
            (:Completed
              (Components|Movement|StopMovementImmediately (Variables|Character|GetCharacterMovement))
              (goto _label))))
        (:then_1
          (CallFunction|Roam))))))

(event OnComponentBeginOverlap(TakedownBox)
  (params (OverlappedComponent :type Primitive%20Component%20Object%20Reference) (OtherActor :type Actor%20Object%20Reference) (OtherComp :type Primitive%20Component%20Object%20Reference) (OtherBodyIndex :type Integer) (bFromSweep :type Boolean) (SweepResult :type Hit%20Result%20Structure%20%28by%20ref%29))
  (if (== OtherActor (Game|GetPlayerCharacter 0))
    (Development|PrintString "Hello")
    (Variables|Default|SetPlayer%20Can%20Takedown true)))

(event OnSeePawn(PawnSensing)
  (params (Pawn :type Pawn%20Object%20Reference))
  ;[1 1 1] Chase Player
  (bind _asbp_top_down_character (Utilities|Casting|CastToBP_TopDownCharacter Pawn))
  (Development|PrintString (Utilities|String|ToString(Boolean) (Variables|/Game/TopDown/Blueprints/BP_TopDownCharacter.BP_TopDownCharacter_C|GetCan%20Be%20Seen _asbp_top_down_character)))
  (if (Variables|/Game/TopDown/Blueprints/BP_TopDownCharacter.BP_TopDownCharacter_C|GetCan%20Be%20Seen _asbp_top_down_character)
    (CallFunction|PlayerIsVisable)))

(event OnComponentEndOverlap(TakedownBox)
  (params (OverlappedComponent :type Primitive%20Component%20Object%20Reference) (OtherActor :type Actor%20Object%20Reference) (OtherComp :type Primitive%20Component%20Object%20Reference) (OtherBodyIndex :type Integer))
  (if (== OtherActor (Game|GetPlayerCharacter 0))
    (Variables|Default|SetPlayer%20Can%20Takedown false)))

(event Custom|follow%20pawn
  ;[1 1 1] Chase Player
  (Variables|Default|SetChasing true)
  (Collision|SetCollisionObjectType (Variables|Collision|GetCapsuleComponent) "ECC_Vehicle")
  (Variables|/Script/Engine.CharacterMovementComponent|SetMaxWalkSpeed (Variables|Character|GetCharacterMovement) 7e+02)
  (AI|AIMoveTo self "0, 0, 0" (Game|GetPlayerCharacter 0) 0.0 false))

(event Custom|Seen%20Target
  (Variables|Default|SetStop%20Chasing false)
  (if (not (Variables|Default|GetStop%20Chasing)) :!label _label
    (CallFunction|FollowPawn)
    (bind _outhit (Collision|LineTraceByChannel (Transformation|GetActorLocation) (Transformation|GetActorLocation (Game|GetPlayerCharacter 0)) "TraceTypeQuery1" false 0 "ForOneFrame" true "(R=1.000000,G=0.000000,B=0.000000,A=1.000000)" "(R=0.000000,G=1.000000,B=0.000000,A=1.000000)" 0.0))
    (if (== (.HitActor (Collision|BreakHitResult _outhit)) (Game|GetPlayerCharacter 0))
      (if (not (Variables|Default|GetStop%20Chasing))
        (Development|PrintString "Hit Player")
        (Utilities|FlowControl|Sequence
          (:then_0
            (goto _label_4 Reset))
          (:then_1
            (Utilities|Time|SetTimerbyEvent (delegate Custom|Roam) 1e+01 :!label _label_2)
            (Development|PrintString "Started Timer"))
          (:then_2
            (Utilities|FlowControl|Delay 0.2 :!label _label_3)
            (goto _label))))
      (else
        (Utilities|FlowControl|Sequence
          (:then_0
            (goto _label_3))
          (:then_1
            (Utilities|FlowControl|DoOnce false :!label _label_4
              (:Completed
                (goto _label_2)))))))))

(event Custom|Player%20is%20Visable
  (if (not (Variables|Default|GetChasing))
    (Variables|Default|SetSeeing%20Pawn true)
    (Components|Movement|StopMovementImmediately (Variables|Character|GetCharacterMovement))
    (if (Collision|IsOverlappingActor (Variables|Default|GetCone) (Game|GetPlayerCharacter 0) :!class /Script/Engine.PrimitiveComponent)
      (CallFunction|FillSuspicion)
      (else
        (CallFunction|DrainSuspicion)))))

(event Custom|Roam
  (Utilities|FlowControl|Sequence
    (:then_0
      (Utilities|FlowControl|DoOnce false) ; enters at Reset
    )
    (:then_1
      (Collision|SetCollisionObjectType (Variables|Collision|GetCapsuleComponent) "ECC_Pawn")
      ;[1 1 1] Roam
      (Variables|Default|SetChasing false)
      (Variables|Default|SetStop%20Chasing true)
      (Variables|/Script/Engine.CharacterMovementComponent|SetMaxWalkSpeed (Variables|Character|GetCharacterMovement) 3e+02)
      (AI|AIMoveTo self (Variables|Default|GetDestination) 0 1e+01 false
        (:OnSuccess
          (CallFunction|Roam))))))

(event Custom|Takedown
  (bind _pawnsensing (Variables|Default|GetPawnSensing))
  (Utilities|FlowControl|DoOnce false
    (:Completed
      (Development|PrintString "Pressed E")
      (if (Variables|Default|GetPlayer%20Can%20Takedown)
        (Collision|SetCollisionEnabled (Variables|Character|GetMesh) "PhysicsOnly")
        (Physics|SetSimulatePhysics (Variables|Character|GetMesh) true)
        (Components|Movement|StopMovementImmediately (Variables|Character|GetCharacterMovement))
        (Pawn|Components|CharacterMovement|DisableMovement (Variables|Character|GetCharacterMovement))
        (Collision|SetCollisionObjectType (Variables|Collision|GetCapsuleComponent) "ECC_WorldDynamic")
        (Components|Tick|SetComponentTickEnabled _pawnsensing false)
        (Variables|/Script/AIModule.PawnSensingComponent|SetbSeePawns _pawnsensing false)))))

(event Custom|Fill%20Suspicion
  (bind _asbp_top_down_character (Utilities|Casting|CastToBP_TopDownCharacter (Game|GetPlayerCharacter 0)))
  (bind _output_get (Variables|Default|SetSuspicion (+ (Variables|Default|GetSuspicion) (Variables|/Game/TopDown/Blueprints/BP_TopDownCharacter.BP_TopDownCharacter_C|GetLight%20Level _asbp_top_down_character))))
  (Development|PrintString (Utilities|String|ToString(Float) _output_get))
  (if (>= _output_get 2.0)
    (Utilities|FlowControl|DoOnce false
      (:Completed
        (Variables|Default|SetSuspicion 0.0)
        (CallFunction|SeenTarget)))))

(event Custom|Drain%20Suspicion
  (Variables|Default|SetSeeing%20Pawn false)
  (if (not (Variables|Default|GetSeeing%20Pawn)) :!label _label
    (if (<= (Variables|Default|GetSuspicion) 0.0)
      (Variables|Default|SetSuspicion 0.0)
      (if (Variables|Default|GetStop%20Chasing)
        (CallFunction|Roam))
      (else
        (Variables|Default|SetSuspicion (- (Variables|Default|GetSuspicion) 1.0))
        (Utilities|FlowControl|Delay 0.5)
        (goto _label)))))

(event EventBeginPlay
  (Utilities|FlowControl|Sequence
    (:then_0
      (Variables|Default|SetDestination (Transformation|GetWorldLocation (Variables|Collision|GetCapsuleComponent)))
      (bind _returnvalue (Game|SpawnActorfromClass "/Game/CustomBlueprints/BP_EnemyFlashlight.BP_EnemyFlashlight_C" (Math|Transform|MakeTransform "0, 0, 0" "0, 0, 0" "1.000000,1.000000,1.000000") "Undefined" "MultiplyWithRoot" 0 0))
      (bind _output_get (Variables|Default|SetFlashlight _returnvalue))
      (Transformation|AttachComponentToComponent _output_get (Variables|Character|GetMesh) "" "KeepRelative" "KeepRelative" "KeepRelative" true))
    (:then_1
      (CallFunction|Roam))))

(fn ConstructionScript)

(fn EnemyList
  (return "NewEnumerator0"))

(fn Interactables
  (return "NewEnumerator0"))