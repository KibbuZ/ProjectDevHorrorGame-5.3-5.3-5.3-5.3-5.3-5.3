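; BP_CubeButton is an interactable world button that starts an interpolated movement when a key is pressed nearby.
; A Sphere overlap shows or hides a Widget component and sets an InRange flag, with no filter on the overlapping actor.
; Pressing E, bound as a debug key event rather than an input action, activates InterpToMovement without reset while InRange is true.
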(event OnComponentBeginOverlap(Sphere)
  (params (OverlappedComponent :type Primitive%20Component%20Object%20Reference) (OtherActor :type Actor%20Object%20Reference) (OtherComp :type Primitive%20Component%20Object%20Reference) (OtherBodyIndex :type Integer) (bFromSweep :type Boolean) (SweepResult :type Hit%20Result%20Structure%20%28by%20ref%29))
  (Rendering|SetVisibility (Variables|Default|GetWidget) true false)
  (Variables|Default|SetinRange true))

(event OnComponentEndOverlap(Sphere)
  (params (OverlappedComponent :type Primitive%20Component%20Object%20Reference) (OtherActor :type Actor%20Object%20Reference) (OtherComp :type Primitive%20Component%20Object%20Reference) (OtherBodyIndex :type Integer))
  (Rendering|SetVisibility (Variables|Default|GetWidget) false false)
  (Variables|Default|SetinRange false))

(event Input|KeyboardEvents|DebugKeyE
  (params (Key :type Key%20Structure :default "None") (ActionValue :type Input%20Action%20Value%20Structure))
  (:Pressed
    (if (Variables|Default|GetinRange)
      (Components|Activation|Activate (Variables|Default|GetInterpToMovement) false))))

(fn ConstructionScript)