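; BP_ActivationOrb is a world-mechanic orb that the player activates by pressing E while in range.
; Actor overlap begin and end toggle a prompt widget and an InRange flag, with no filter on the overlapping actor.
; An E debug key event checks that flag, then shows one light and sphere pair and hides the other.
; The swap is purely visual and one-way.
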(event Collision|EventActorBeginOverlap
  (params (OtherActor :type Actor%20Object%20Reference))
  (Rendering|SetVisibility (Variables|Default|GetWidget) true false)
  (Variables|Default|SetinRange true))

(event Collision|EventActorEndOverlap
  (params (OtherActor :type Actor%20Object%20Reference))
  (Rendering|SetVisibility (Variables|Default|GetWidget) false false)
  (Variables|Default|SetinRange false))

(event Input|KeyboardEvents|DebugKeyE
  (params (Key :type Key%20Structure :default "None") (ActionValue :type Input%20Action%20Value%20Structure))
  (:Pressed
    (if (Variables|Default|GetinRange)
      (Rendering|SetVisibility (Variables|Default|GetPointLight) true false)
      (Rendering|SetVisibility (Variables|Default|GetSphere) true false)
      (Rendering|SetVisibility (Variables|Default|GetPointLight1) false false)
      (Rendering|SetVisibility (Variables|Default|GetSphere2) false false))))

(fn ConstructionScript)