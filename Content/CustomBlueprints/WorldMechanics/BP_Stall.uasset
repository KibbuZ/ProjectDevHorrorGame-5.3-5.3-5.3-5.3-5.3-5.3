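; BP_Stall is an interactable stall that the player can hide in.
; A box overlap shows the interact prompt and enables Interact, which flip-flops between teleporting the player inside and out in front, toggling IsHiding on BP_TopDownCharacter.
; Entering also plays a sound and emits a long-range AI noise offset along the stall's forward vector, away from the player's position.
; EnemyList, HidingPlaces and Interactables each return a fixed enum value.
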(event OnComponentBeginOverlap(Box)
  (params (OverlappedComponent :type Primitive%20Component%20Object%20Reference) (OtherActor :type Actor%20Object%20Reference) (OtherComp :type Primitive%20Component%20Object%20Reference) (OtherBodyIndex :type Integer) (bFromSweep :type Boolean) (SweepResult :type Hit%20Result%20Structure%20%28by%20ref%29))
  (if (== OtherActor (Game|GetPlayerCharacter 0))
    (Development|SetHiddeninGame (Variables|Default|GetInteract%20Prompt) false false)
    (Variables|Default|SetPlayer%20Overlapping true)))

(event OnComponentEndOverlap(Box)
  (params (OverlappedComponent :type Primitive%20Component%20Object%20Reference) (OtherActor :type Actor%20Object%20Reference) (OtherComp :type Primitive%20Component%20Object%20Reference) (OtherBodyIndex :type Integer))
  (if (== OtherActor (Game|GetPlayerCharacter 0))
    (Development|SetHiddeninGame (Variables|Default|GetInteract%20Prompt) true false)
    (Variables|Default|SetPlayer%20Overlapping false)))

(event Custom|Interact
  (bind _returnvalue (Game|GetPlayerCharacter 0))
  (bind _box (Variables|Default|GetBox))
  (bind _defaultsceneroot (Variables|Default|GetDefaultSceneRoot))
  (if (Variables|Default|GetPlayer%20Overlapping)
    (Utilities|FlowControl|FlipFlop
      (:A
        (Transformation|Teleport (Game|GetPlayerCharacter 0) (Transformation|GetWorldLocation (Variables|Default|GetBox)) "0, 0, 0")
        (Audio|PlaySound2D "/Engine/EditorSounds/GamePreview/PossessPlayer_Cue.PossessPlayer_Cue" 1.0 1.0 0.0 0 0)
        (Class|Actor|MakeNoise 1.0 _returnvalue (+ (* (Math|Vector|GetForwardVector (Transformation|GetWorldRotation _defaultsceneroot)) 5e+02) (Transformation|GetWorldLocation _defaultsceneroot)) 1e+05 "None")
        (bind _asbp_top_down_character (Utilities|Casting|CastToBP_TopDownCharacter _returnvalue))
        (Variables|/Game/TopDown/Blueprints/BP_TopDownCharacter.BP_TopDownCharacter_C|SetIs%20Hiding _asbp_top_down_character true))
      (:B
        (Transformation|Teleport (Game|GetPlayerCharacter 0) (+ (Transformation|GetWorldLocation _box) (* (Math|Vector|GetForwardVector (Transformation|GetWorldRotation _box)) 1e+02)) (Transformation|GetWorldRotation (Variables|Default|GetBox)))
        (bind _asbp_top_down_character_2 (Utilities|Casting|CastToBP_TopDownCharacter (Game|GetPlayerCharacter 0)))
        (Variables|/Game/TopDown/Blueprints/BP_TopDownCharacter.BP_TopDownCharacter_C|SetIs%20Hiding _asbp_top_down_character_2 false)))))

(fn ConstructionScript)

(fn EnemyList
  (return "NewEnumerator6"))

(fn HidingPlaces
  (return "NewEnumerator7"))

(fn Interactables
  (return "NewEnumerator1"))