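; BP_SaveCloset is a hiding closet the player can get into and out of with E or Shift+E debug keys.
; Player overlap sets an in-range flag and shows a widget; a FlipFlop then alternates teleporting into the box or just in front of it, toggling IsHiding on BP_TopDownCharacter.
; Entering also plays a sound and emits a long-range AI noise ahead of the closet.
; Small functions return enum values for enemy, hiding-place and interactable categories.
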(event Collision|EventActorBeginOverlap
  (params (OtherActor :type Actor%20Object%20Reference))
  ;[1 1 1] Detect if player is in range of closet to enter the closet
  (if (== OtherActor (Game|GetPlayerCharacter 0))
    (Variables|Default|SetIn%20Range true)
    (Rendering|SetVisibility (Variables|Default|GetWidget) true false)))

(event Collision|EventActorEndOverlap
  (params (OtherActor :type Actor%20Object%20Reference))
  ;[1 1 1] Detect if player is in range of closet to enter the closet
  (if (== (Game|GetPlayerCharacter 0) OtherActor)
    (Variables|Default|SetIn%20Range false)
    (Rendering|SetVisibility (Variables|Default|GetWidget) false false)))

(event Input|KeyboardEvents|DebugKeyE
  (params (Key :type Key%20Structure :default "None") (ActionValue :type Input%20Action%20Value%20Structure))
  (bind _returnvalue (Game|GetPlayerCharacter 0))
  (bind _box (Variables|Default|GetBox))
  (bind _defaultsceneroot (Variables|Default|GetDefaultSceneRoot))
  ;[1 1 1] Get in and out of the Closet
  (:Pressed
    (if (Variables|Default|GetIn%20Range)
      (Utilities|FlowControl|FlipFlop
        (:A
          (Transformation|Teleport (Game|GetPlayerCharacter 0) (Transformation|GetWorldLocation (Variables|Default|GetBox)) "0, 0, 0")
          (Audio|PlaySound2D "/Engine/EditorSounds/GamePreview/PossessPlayer_Cue.PossessPlayer_Cue" 1.0 1.0 0.0 0 0)
          (Class|Actor|MakeNoise 1.0 _returnvalue (+ (* (Math|Vector|GetForwardVector (Transformation|GetWorldRotation _defaultsceneroot)) 5e+02) (Transformation|GetWorldLocation _defaultsceneroot)) 1e+05 "None")
          (bind _asbp_top_down_character (Utilities|Casting|CastToBP_TopDownCharacter _returnvalue))
          (Variables|/Game/TopDown/Blueprints/BP_TopDownCharacter.BP_TopDownCharacter_C|SetIs%20Hiding _asbp_top_down_character true))
        (:B
          (Transformation|Teleport (Game|GetPlayerCharacter 0) (+ (Transformation|GetWorldLocation _box) (* (Math|Vector|GetForwardVector (Transformation|GetWorldRotation _box)) 1e+02)) (Transformation|GetWorldRotation (Variables|Default|GetBox)))
          (bind _asbp_top_down_character_2 (Utilities|Casting|CastToBP_TopDownCharacter (Game|GetPlayerCharacter 0)))
          (Variables|/Game/TopDown/Blueprints/BP_TopDownCharacter.BP_TopDownCharacter_C|SetIs%20Hiding _asbp_top_down_character_2 false))))))

(event Input|KeyboardEvents|DebugKeyShiftE
  (params (Key :type Key%20Structure :default "None") (ActionValue :type Input%20Action%20Value%20Structure))
  (bind _returnvalue (Game|GetPlayerCharacter 0))
  (bind _box (Variables|Default|GetBox))
  (bind _defaultsceneroot (Variables|Default|GetDefaultSceneRoot))
  ;[1 1 1] Get in and out of the Closet
  (:Pressed
    (if (Variables|Default|GetIn%20Range)
      (Utilities|FlowControl|FlipFlop
        (:A
          (Transformation|Teleport (Game|GetPlayerCharacter 0) (Transformation|GetWorldLocation (Variables|Default|GetBox)) "0, 0, 0")
          (Audio|PlaySound2D "/Engine/EditorSounds/GamePreview/PossessPlayer_Cue.PossessPlayer_Cue" 1.0 1.0 0.0 0 0)
          (Class|Actor|MakeNoise 1.0 _returnvalue (+ (* (Math|Vector|GetForwardVector (Transformation|GetWorldRotation _defaultsceneroot)) 5e+02) (Transformation|GetWorldLocation _defaultsceneroot)) 1e+05 "None")
          (bind _asbp_top_down_character (Utilities|Casting|CastToBP_TopDownCharacter _returnvalue))
          (Variables|/Game/TopDown/Blueprints/BP_TopDownCharacter.BP_TopDownCharacter_C|SetIs%20Hiding _asbp_top_down_character true))
        (:B
          (Transformation|Teleport (Game|GetPlayerCharacter 0) (+ (Transformation|GetWorldLocation _box) (* (Math|Vector|GetForwardVector (Transformation|GetWorldRotation _box)) 1e+02)) (Transformation|GetWorldRotation (Variables|Default|GetBox)))
          (bind _asbp_top_down_character_2 (Utilities|Casting|CastToBP_TopDownCharacter (Game|GetPlayerCharacter 0)))
          (Variables|/Game/TopDown/Blueprints/BP_TopDownCharacter.BP_TopDownCharacter_C|SetIs%20Hiding _asbp_top_down_character_2 false))))))

(fn ConstructionScript)

(fn NewFunction
  (params (InDouble :type Float%20%28double-precision%29%20%28by%20ref%29) (NewParam :type Float%20%28double-precision%29%20%28by%20ref%29) (NewParam1 :type Float%20%28double-precision%29%20%28by%20ref%29) (NewParam2 :type Vector%20%28by%20ref%29))
  (return (Math|Conversions|ToVector(Float) InDouble)))

(fn EnemyList
  (return "NewEnumerator6"))

(fn HidingPlaces
  (return "NewEnumerator1"))

(fn Interactables
  (return "NewEnumerator1"))